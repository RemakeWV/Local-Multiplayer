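; Player character that carries up to two boxes, stores them in a truck for points, and can move, jump, attack and pause.
; Storing lerps each box to the truck point via a timeline before destroying it, then adds the box count to the score widget.
; BeginPlay gives body, head and score widget a shared random color through a dynamic material.
; Attacking while overlapping other players triggers box drops and clears the carry slots.
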(event `StoreBoxes`
  (params (Truck :type "/Game/02-Blueprints/Truck_BP Object Reference"))
  ;[1 1 1] Store Boxes
  (bind _boxone (`self.BoxOne`)
    (:`then`
      (`GameplayStatics.PlaySound2D` "/Game/06-Sounds/PositiveBass_Cue.PositiveBass_Cue" (`/Game/02-Blueprints/Data/GameInfo.MasterVolume` (`/Game/02-Blueprints/Data/BFL.Get Game Info`)) 1.0 0.0 null null)
      (`self.SendToBack` _boxone Truck))
    (:`else`
      _))
  (`KismetSystemLibrary.Delay` 0.3)
  (bind _boxtwo (`self.BoxTwo`)
    (:`then`
      (`GameplayStatics.PlaySound2D` "/Game/06-Sounds/PositiveBass_Cue.PositiveBass_Cue" (`/Game/02-Blueprints/Data/GameInfo.MasterVolume` (`/Game/02-Blueprints/Data/BFL.Get Game Info`)) 1.0 0.0 null null)
      (`self.SendToBack` _boxtwo Truck))
    (:`else`
      _))
  (`self.UpdateScore` (`self.Boxes`))
  (`self.ClearBoxes`))

(event `SendToBack`
  (params (Box :type "/Game/02-Blueprints/Box_BP Object Reference") (Truck :type "/Game/02-Blueprints/Truck_BP Object Reference"))
  (bind _box (`/Game/02-Blueprints/Box_BP.Box` Box))
  (bind (_direction _lerp) (`Timeline|Lerp` :!via `PlayFromStart`)
    (:`Update`
      (`SceneComponent.K2_SetWorldLocation` _box (`KismetMathLibrary.VLerp` (`SceneComponent.K2_GetComponentLocation` _box) (`SceneComponent.K2_GetComponentLocation` (`/Game/02-Blueprints/Truck_BP.TruckPoint` Truck)) _lerp) false false))
    (:`Finished`
      (`self.K2_DestroyActor` Box))))

(event `self.ReceiveBeginPlay`
  (bind _body (`self.Body`))
  (bind _returnvalue (`PrimitiveComponent.CreateDynamicMaterialInstance` _body 0 (`PrimitiveComponent.GetMaterial` _body 0) "None"))
  (set `self.PlayerMaterial` _returnvalue)
  (set `self.Color` (`KismetMathLibrary.MakeColor` (`KismetMathLibrary.RandomFloatInRange` 0.1 1.0) (`KismetMathLibrary.RandomFloatInRange` 0.1 1.0) (`KismetMathLibrary.RandomFloatInRange` 0.1 1.0)))
  (`MaterialInstanceDynamic.SetVectorParameterValue` (`self.PlayerMaterial`) "Color" (`self.Color`))
  (`PrimitiveComponent.SetMaterial` (`self.Head`) 0 (`self.PlayerMaterial`))
  (`PrimitiveComponent.SetMaterial` (`self.Body`) 0 (`self.PlayerMaterial`))
  (bind _asplayer_points (cast `/Game/08-UI/PlayerPoints` (`WidgetComponent.GetUserWidgetObject` (`self.Widget`))))
  (bind _output_get (set `self.PlayerScoreWidget` _asplayer_points))
  (`UserWidget.SetColorAndOpacity` _output_get (`self.Color`)))

(event `InputAction|Pause`
  (params (Key :type "Key Structure"))
  (:`Pressed`
    (`/Game/02-Blueprints/GameModes/Game_GM.PauseGame` (`/Game/02-Blueprints/Data/BFL.GetGM`))))

(event `InputAxis|MoveUp`
  (params (AxisValue :type "Float (single-precision)"))
  ;[1 1 1] Movement
  (`self.AddMovementInput` (`SceneComponent.GetRightVector` (`self.CapsuleComponent`)) AxisValue))

(event `InputAction|Jump`
  (params (Key :type "Key Structure"))
  (:`Pressed`
    (`self.Jump`)
    (if (not (`NavMovementComponent.IsFalling` (`self.CharacterMovement`)))
      (`GameplayStatics.PlaySound2D` "/Game/06-Sounds/JumpNoise_Cue.JumpNoise_Cue" (`/Game/02-Blueprints/Data/GameInfo.MasterVolume` (`/Game/02-Blueprints/Data/BFL.Get Game Info`)) 1.0 0.0 null null))))

(event `InputAxis|MoveRight`
  (params (AxisValue :type "Float (single-precision)"))
  ;[1 1 1] Movement
  (`self.AddMovementInput` (`SceneComponent.GetForwardVector` (`self.CapsuleComponent`)) AxisValue))

(event `UpdateScore`
  (params (Points :type Integer))
  (bind _playerscorewidget (`self.PlayerScoreWidget`))
  ;[1 1 1] Update the Score
  (set `/Game/08-UI/PlayerPoints.Points` (+ Points (`/Game/08-UI/PlayerPoints.Points` _playerscorewidget)) _playerscorewidget))

(event `InputAction|Attack`
  (params (Key :type "Key Structure"))
  ;[1 1 1] Attack
  (:`Pressed`
    (set `self.Attacking?` true)
    (for _array_element (`self.GetOverlappingActors` "Player_BP_C")
      (`self.DropMyBoxes`)
      (`/Engine/EditorBlueprintResources/StandardMacros.IsValid` _array_element
        (:`Is Valid`
          (`self.DropMyBoxes`))
        (:`Is Not Valid`
          _))
      (`self.ClearBoxes`)))
  (:`Released`
    (set `self.Attacking?` false)))

(event `DropMyBoxes`
  ;[1 1 1] Drop my boxes
  (bind _boxone (`self.BoxOne`)
    (:`then`
      (`/Game/02-Blueprints/Box_BP.DropIt` _boxone))
    (:`else`
      _))
  (bind _boxtwo (`self.BoxTwo`)
    (:`then`
      (`/Game/02-Blueprints/Box_BP.DropIt` _boxtwo))
    (:`else`
      _))
  (`self.ClearBoxes`))

(fn `ClearBoxes`
  (set `self.Boxes` 0)
  (set `self.BoxOne` null)
  (set `self.BoxTwo` null))

(fn `UserConstructionScript`)